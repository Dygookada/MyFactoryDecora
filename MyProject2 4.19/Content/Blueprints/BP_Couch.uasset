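; BP_Couch is a couch actor whose look is built from an array of static mesh components.
; Its construction script loops up to IntStaticMesh, assigning each component the mesh at the same index in the NewVar00 array.
; BeginPlay runs the parent logic, then calls SetArrayMesh, which is defined outside this file.
; Overlap and Tick events are disabled.
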(event `self.ReceiveBeginPlay`
  (`parent.ReceiveBeginPlay`)
  (`self.SetArrayMesh`))

(fn `UserConstructionScript`
  (`parent.UserConstructionScript`)
  (for _index (range (+ (`self.Int_StaticMesh`) 1))
    (`StaticMeshComponent.SetStaticMesh` (`|GetArrayItem` (`self.StaticMeshComponent`) _index) (`|GetArrayItem` (`self.NewVar_0_0`) _index))))