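; Interactable actor that lets the first-person player open a menu and swap its static mesh.
; A sphere registers the actor as a player target and shows a name label that turns toward the player's camera.
; Interaction toggles the animated menu, mouse cursor and input mode, blending the view between actor and pawn.
; Change applies a mesh by index from a GameMode array chosen by InformationType.
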(event `MenuObject`
  (params (Target :type "/Game/Blueprints/W_MenuObj Object Reference"))
  (bind _returnvalue (`GameplayStatics.GetPlayerController` 0))
  (bind _open (`/Game/Blueprints/W_MenuObj.Open` Target))
  ;[0 0 0] Importante
  (set `/Game/Blueprints/W_MenuObj.ReferenceActor` self Target)
  (`self.SetArrayMesh`)
  (set `/Game/Blueprints/W_MenuObj.Length` (`KismetArrayLibrary.Array_LastIndex` (`self.ArrayMesh`)) Target)
  (`/Engine/EditorBlueprintResources/StandardMacros.FlipFlop`
    (:`A`
      (`UserWidget.AddToViewport` Target 0)
      (`self.OpenMenuSetObject` Target _open _returnvalue :!pinned true) ; Para poder ter os eventos de tela disponiveis
    )
    (:`B`
      (`self.CloseMenuSetObject` Target _open _returnvalue :!pinned true) ; Para poder ter os movimentos de mouse disponiveis de novo
      (`KismetSystemLibrary.Delay` 0.5)
      (`Widget.RemoveFromParent` Target))))

(event `self.ReceiveBeginPlay`
  (`self.SetArrayMesh`))

(event `self.ReceiveTick`
  (params (DeltaSeconds :type "Float (single-precision)"))
  (bind _0123 (`self.0123`))
  ;[1 1 1] Detectar aproximacao
  (if (stale `self.Sphere.OnComponentBeginOverlap` bFromSweep) :!pinned true
    (`SceneComponent.K2_SetWorldRotation` _0123 (`KismetMathLibrary.FindLookAtRotation` (`SceneComponent.K2_GetComponentLocation` _0123) (`SceneComponent.K2_GetComponentLocation` (`/Game/FirstPersonBP/Blueprints/FirstPersonCharacter.FirstPersonCamera` (stale `self.Sphere.OnComponentBeginOverlap` _asfirst_person_character)))) false false :!pinned true) ; Deixa o nome sempre na frente do player
  ))

(event `self.Sphere.OnComponentBeginOverlap`
  (params (OverlappedComponent :type "PrimitiveComponent Object Reference") (OtherActor :type "Actor Object Reference") (OtherComp :type "PrimitiveComponent Object Reference") (OtherBodyIndex :type Integer) (bFromSweep :type Boolean) (SweepResult :type "HitResult Structure (by ref)"))
  ;[1 1 1] Detectar aproximacao
  ;;[1 1 1] Adicionar os objetos interativos
  (bind _asfirst_person_character (cast `/Game/FirstPersonBP/Blueprints/FirstPersonCharacter` OtherActor))
  (`KismetArrayLibrary.Array_Add` (`/Game/FirstPersonBP/Blueprints/FirstPersonCharacter.TargetActor` _asfirst_person_character) self)
  ;;[1 1 1] Ativar e desativar o nome
  (`SceneComponent.SetVisibility` (`self.0123`) true false))

(event `self.Sphere.OnComponentEndOverlap`
  (params (OverlappedComponent :type "PrimitiveComponent Object Reference") (OtherActor :type "Actor Object Reference") (OtherComp :type "PrimitiveComponent Object Reference") (OtherBodyIndex :type Integer))
  ;[1 1 1] Detectar aproximacao
  ;;[1 1 1] Adicionar os objetos interativos
  (bind _asfirst_person_character (cast `/Game/FirstPersonBP/Blueprints/FirstPersonCharacter` OtherActor))
  (`KismetArrayLibrary.Array_RemoveItem` (`/Game/FirstPersonBP/Blueprints/FirstPersonCharacter.TargetActor` _asfirst_person_character) self)
  ;;[1 1 1] Ativar e desativar o nome
  (`SceneComponent.SetVisibility` (`self.0123`) false false))

(event `Interaction`
  (params (Menu :type "/Game/Blueprints/W_MenuObj Object Reference") (RefPlayer :type "/Game/FirstPersonBP/Blueprints/FirstPersonCharacter Object Reference"))
  (bind _returnvalue (`GameplayStatics.GetPlayerController` 0))
  (set `self.Menu` Menu)
  (`self.MenuObject` Menu)
  (`/Engine/EditorBlueprintResources/StandardMacros.FlipFlop`
    (:`A`
      (`PlayerController.SetViewTargetWithBlend` _returnvalue self 0.5 "VTBlend_Linear" 0.0 false))
    (:`B`
      (`PlayerController.SetViewTargetWithBlend` _returnvalue (cast `/Game/FirstPersonBP/Blueprints/FirstPersonCharacter` (`GameplayStatics.GetPlayerPawn` 0) :!pure true) 0.5 "VTBlend_Linear" 0.0 false))))

(event `Color`)

(event `Change`
  (params (Integer :type Integer) (Object :type Name))
  (set `self.IndexInfo` Integer)
  (`StaticMeshComponent.SetStaticMesh` (`self.StaticMesh`) (`.Mesh_11_7A6020580C42DC73E8252D96C154BDB7` (break `/Game/Blueprints/Details/MenuInfoMesh` (`|GetArrayItem` (`self.ArrayMesh`) Integer)))))

(fn `CloseMenuSetObject`
  (params (Menu :type "UserWidget Object Reference") (InAnimation :type "WidgetAnimation Object Reference") (PlayerControl :type "PlayerController Object Reference"))
  (set `PlayerController.bShowMouseCursor` false PlayerControl)
  (`UserWidget.PlayAnimation` Menu InAnimation 0.0 1 "Reverse" 2.0)
  (`WidgetBlueprintLibrary.SetInputMode_GameOnly` PlayerControl) ; Por isso recolocar o mode game only
)

(fn `HowManyStaticMesh`
  (for _index (range (+ (`self.Int_StaticMesh`) 1))
    (bind _returnvalue (`AddComponent|NODE_AddStaticMeshComponent-5` :`bManualAttachment` true :`RelativeTransform` (`SceneComponent.GetRelativeTransform` (`self.DefaultSceneRoot`))))
    (`KismetArrayLibrary.Array_Set` (`self.StaticMeshComponent`) _index _returnvalue true))
  (return))

(fn `OnRep_Menu`)

(fn `OpenMenuSetObject`
  (params (Menu :type "UserWidget Object Reference") (InAnimation :type "WidgetAnimation Object Reference") (PlayerControl :type "PlayerController Object Reference"))
  (set `PlayerController.bShowMouseCursor` true PlayerControl)
  (`UserWidget.PlayAnimation` Menu InAnimation 0.0 1 "Forward" 2.0)
  (`WidgetBlueprintLibrary.SetInputMode_GameAndUIEx` PlayerControl Menu) ; Para poder ter os eventor de tela disponiveis
)

(fn `SetArrayMesh`
  (bind _asfirst_person_game_mode (cast `/Game/FirstPersonBP/Blueprints/FirstPersonGameMode` (`GameplayStatics.GetGameMode`)))
  (set `self.ArrayMesh` (`/Game/FirstPersonBP/Blueprints/FirstPersonGameMode.Select` _asfirst_person_game_mode (`self.InformationType`))))

(fn `UserConstructionScript`
  (`self.SetArrayMesh`)
  (`SphereComponent.SetSphereRadius` (`self.Sphere`) (`self.ContactArea`) true)
  (`TextRenderComponent.K2_SetText` (`self.0123`) (`self.Name`)))